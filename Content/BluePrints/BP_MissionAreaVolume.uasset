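; BP_MissionAreaVolume is a boundary volume that punishes the player for leaving the mission area.
; When a BP_Marine exits, it flags the marine as outside, starts a camera and audio fade to a dark tint, and runs a looping KillPlayer timer.
; KillPlayer repeatedly damages player character 0, whichever marine triggered it.
; Re-entering clears the flag, timer and fade.
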(event Collision|EventActorBeginOverlap
  (params (OtherActor :type Actor%20Object%20Reference))
  (bind _asbp_marine (Utilities|Casting|CastToBP_Marine OtherActor))
  (Variables|/Game/BluePrints/Pawns/BP_Marine.BP_Marine_C|SetisOutsideMissionArea _asbp_marine false)
  (Utilities|Time|ClearTimerbyFunctionName 0 "KillPlayer")
  (CameraFades|StopCameraFade (Game|GetPlayerCameraManager 0)))

(event Collision|EventActorEndOverlap
  (params (OtherActor :type Actor%20Object%20Reference))
  (bind _asbp_marine (Utilities|Casting|CastToBP_Marine OtherActor))
  (Variables|/Game/BluePrints/Pawns/BP_Marine.BP_Marine_C|SetisOutsideMissionArea _asbp_marine true)
  (Utilities|Time|SetTimerbyFunctionName 0 "KillPlayer" 0.7 true)
  (CameraFades|StartCameraFade (Game|GetPlayerCameraManager 0) 0.0 0.75 1.7 "(R=0.035417,G=0.018313,B=0.005977,A=1.000000)" true true))

(fn ConstructionScript)

(fn KillPlayer
  (Game|Damage|ApplyDamage (Game|GetPlayerCharacter 0) 1e+01 0 0))