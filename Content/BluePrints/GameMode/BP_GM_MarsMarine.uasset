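; Game mode for Mars Marine that runs endless, escalating waves of BP_Alien enemies.
; Each wave multiplies the difficulty to set its spawn count, then a looping timer spawns aliens at random TargetPoints until none remain to spawn.
; Spawned aliens are tracked in an array; RegistareAlienDeath removes them and, once the wave is cleared, starts the next after a short delay.
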(event Custom|Spawn%20Event
  (CallFunction|SpawnAlien))

(event Custom|End%20Wave
  (Utilities|FlowControl|Delay 3.0)
  (CallFunction|SetupNewWave))

(event EventBeginPlay
  (Utilities|FlowControl|Delay 1.3)
  (CallFunction|SetupNewWave))

(fn ConstructionScript)

(fn SetupNewWave
  (Math|Integer|IncrementInt (Variables|Default|GetcurrentWave)
    (:%20%20
      (CallFunction|IncreaseWaveDifficulty)
      (Utilities|Time|SetTimerbyFunctionName 0 "Spawn Event" 1.3 true))))

(fn SpawnAlien
  (bind _output (CallFunction|GetRandomSpawnPoint))
  (Utilities|IsValid _output
    (:Is%20Valid
      (bind _returnvalue (Game|SpawnActorfromClass "/Game/BluePrints/Pawns/BP_Alien.BP_Alien_C" (Transformation|GetActorTransform _output) "Undefined" "MultiplyWithRoot" 0 0))
      (Utilities|IsValid _returnvalue
        (:Is%20Valid
          (Utilities|Array|Add (Variables|Default|GetAliens) _returnvalue)
          (bind _result (Math|Integer|DecrementInt (Variables|Default|GetAlienSpawnsRemaining))
            (:%20%20
              (if (== _result 0)
                (Utilities|Time|ClearTimerbyFunctionName 0 "Spawn Event")))))))))

(fn GetRandomSpawnPoint
  (bind _outactors (Actor|GetAllActorsOfClass "/Script/Engine.TargetPoint"))
  (return (Utilities|Array|Get(acopy) _outactors (Math|Random|RandomIntegerinRange 0 (Utilities|Array|LastIndex _outactors)))))

(fn RegistareAlienDeath
  (params (deathAlien :type BP%20Alien%20Object%20Reference%20%28by%20ref%29))
  (Utilities|Array|RemoveItem (Variables|Default|GetAliens) deathAlien)
  (if (CallFunction|IsWaveIsComplete)
    (CallFunction|EndWave)))

(fn IsWaveIsComplete
  (return (and (== (Utilities|Array|Length (Variables|Default|GetAliens)) 0) (== (Variables|Default|GetAlienSpawnsRemaining) 0))))

(fn IncreaseWaveDifficulty
  (bind _output_get (Variables|Default|SetwaveDifficulty (Math|Float|Round (* (Variables|Default|GetwaveDifficulty) (Variables|Default|GetdifficultyMultiplier)))))
  (Variables|Default|SetAlienSpawnsRemaining _output_get))