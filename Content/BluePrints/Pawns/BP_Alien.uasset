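; BP_Alien is an enemy pawn that chases the player marine and claws it until killed.
; A repeating AIMoveTo loop drives pursuit, while Tick plays the attack montage when in range and not already playing it.
; Left and right claw overlaps damage the player while CanDamage is set.
; Lethal damage stops movement and collision, credits the marine's kill, notifies the game mode, then destroys the alien after a delay.
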(event OnComponentBeginOverlap(L_ClawCollider)
  (params (OverlappedComponent :type Primitive%20Component%20Object%20Reference) (OtherActor :type Actor%20Object%20Reference) (OtherComp :type Primitive%20Component%20Object%20Reference) (OtherBodyIndex :type Integer) (bFromSweep :type Boolean) (SweepResult :type Hit%20Result%20Structure%20%28by%20ref%29))
  (Utilities|Casting|CastToBP_Marine OtherActor)
  (if (Variables|Default|GetcanDamage)
    (CallFunction|DamagePlayer)))

(event OnComponentBeginOverlap(R_ClawCollider)
  (params (OverlappedComponent :type Primitive%20Component%20Object%20Reference) (OtherActor :type Actor%20Object%20Reference) (OtherComp :type Primitive%20Component%20Object%20Reference) (OtherBodyIndex :type Integer) (bFromSweep :type Boolean) (SweepResult :type Hit%20Result%20Structure%20%28by%20ref%29))
  (Utilities|Casting|CastToBP_Marine OtherActor)
  (if (Variables|Default|GetcanDamage)
    (CallFunction|DamagePlayer)))

(event EventBeginPlay
  (AI|AIMoveTo self "0, 0, 0" (Game|GetPlayerCharacter 0) 11.0 false :!label _label
    (:OnSuccess
      _)
    (:OnFail
      _))
  (Utilities|FlowControl|Delay 0.3)
  (if (CallFunction|IsAlienAlive)
    (goto _label)))

(event Game|Damage|EventAnyDamage
  (params (Damage :type Float%20%28single-precision%29) (DamageType :type Damage%20Type%20Object%20Reference) (InstigatedBy :type Controller%20Object%20Reference) (DamageCauser :type Actor%20Object%20Reference))
  (if (CallFunction|IsAlienAlive)
    (bind _currenthealth (CallFunction|DecreaseHealth Damage))
    (if (<= _currenthealth 0.0)
      (CallFunction|ProcessDeath)
      (Utilities|FlowControl|Delay 1.7)
      (Actor|DestroyActor))))

(event EventTick
  (params (DeltaSeconds :type Float%20%28single-precision%29))
  (if (CallFunction|CanAttack)
    (Animation|Montage|PlayMontage (Variables|Character|GetMesh) "/Game/Characters/Enemy_Great_Spider/Animations/SA_Attacktack_AM.SA_Attacktack_AM")))

(fn ConstructionScript)

(fn IsinAttackRange
  (return (<= (Transformation|GetDistanceTo (Game|Player|GetPlayerPawn 0)) (Variables|Default|GetattackRange))))

(fn IsAttacking
  (return (not (Animation|Montage|MontageIsPlaying (Components|SkeletalMesh|GetAnimInstance (Variables|Character|GetMesh)) "/Game/Characters/Enemy_Great_Spider/Animations/SA_Attacktack_AM.SA_Attacktack_AM"))))

(fn DamagePlayer
  (if (CallFunction|IsAlienAlive)
    (Game|Damage|ApplyDamage (Game|GetPlayerCharacter 0) (Variables|Default|GetdamagePerHit) 0 0)))

(fn DecreaseHealth
  (params (Damage :type Float%20%28double-precision%29))
  (bind _output_get (Variables|Default|Sethealth (- (Variables|Default|Gethealth) Damage)))
  (return _output_get))

(fn ProcessDeath
  (bind _charactermovement (Variables|Character|GetCharacterMovement))
  (Variables|Default|SetisDead true)
  (Components|Movement|StopMovementImmediately _charactermovement)
  (Components|Activation|Deactivate _charactermovement)
  (Collision|SetActorEnableCollision false)
  (bind _asbp_marine (Utilities|Casting|CastToBP_Marine (Game|GetPlayerCharacter 0)))
  (Default|IncreaseKills _asbp_marine)
  (bind _asbp_gm_mars_marine (Utilities|Casting|CastToBP_GM_MarsMarine (Game|GetGameMode)))
  (Default|RegistareAlienDeath _asbp_gm_mars_marine self))

(fn IsAlienAlive
  (return (not (Variables|Default|GetisDead))))

(fn CanAttack
  (return (Math|Boolean|ANDBoolean (CallFunction|IsinAttackRange) (CallFunction|IsAttacking) (CallFunction|IsAlienAlive))))